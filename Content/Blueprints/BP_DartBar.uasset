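; BP_DartBar is an oscillating bar, apparently a timing meter for a dart game, that the player stops with the X key.
; BeginPlay starts a delay loop, timed by PlayRate, that alternately plays DartBarTimeline forward and in reverse through GoUpDown.
; The timeline update lerps Cube1's relative Z position toward Height.
; Pressing X stores Cube1's Z, sets Done to block further swings, calls CallDone and stops the timeline.
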(event Custom|GoUp
  (bind _newtrack_0 (Timeline|DartBarTimeline PlayFromStart)
    (:Update
      (Transformation|SetRelativeLocation (Variables|Default|GetCube1) (Math|Vector|Lerp(Vector) "0, 0, 0" (Math|Vector|MakeVector 0.0 0.0 (Variables|Default|GetHeight)) _newtrack_0) false false))))

(event Custom|GoDown
  (bind _newtrack_0 (Timeline|DartBarTimeline ReverseFromEnd)
    (:Update
      (Transformation|SetRelativeLocation (Variables|Default|GetCube1) (Math|Vector|Lerp(Vector) "0, 0, 0" (Math|Vector|MakeVector 0.0 0.0 (Variables|Default|GetHeight)) _newtrack_0) false false))))

(event EventBeginPlay
  (Components|Timeline|SetPlayRate (Variables|Default|GetDartBarTimeline) (Variables|Default|GetPlayRate))
  (CallFunction|GoUpDown :!label _label)
  (Utilities|FlowControl|Delay (/ 1.0 (Variables|Default|GetPlayRate)))
  (goto _label))

(event Collision|EventActorBeginOverlap
  (params (OtherActor :type Actor%20Object%20Reference)))

(event EventTick
  (params (DeltaSeconds :type Float%20%28single-precision%29)))

(event Input|KeyboardEvents|X
  (params (Key :type Key%20Structure :default "None"))
  (:Pressed
    (Variables|Default|SetRelative%20Location%20Z (.z (Variables|/Script/Engine.SceneComponent|GetRelativeLocation (Variables|Default|GetCube1))))
    (Development|PrintString "Hello")
    (Variables|Default|SetDone? true)
    (Default|CallDone)
    (bind _newtrack_0 (Timeline|DartBarTimeline Stop)
      (:Update
        (Transformation|SetRelativeLocation (Variables|Default|GetCube1) (Math|Vector|Lerp(Vector) "0, 0, 0" (Math|Vector|MakeVector 0.0 0.0 (Variables|Default|GetHeight)) _newtrack_0) false false)))))

(fn ConstructionScript)

(fn GoUpDown
  (if (not (Variables|Default|GetDone?))
    (if (Variables|Default|GetGoingUp)
      (CallFunction|GoUp)
      (Variables|Default|SetGoingUp false)
      (else
        (CallFunction|GoDown)
        (Variables|Default|SetGoingUp true)))))