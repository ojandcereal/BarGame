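; BP_Darts is a darts minigame actor that chains two BP_DartBar child actors, horizontal then vertical, to trigger a dart throw.
; Each bar receives player input in turn, and its Done event advances the sequence while recording its position.
; The final step calls the first-person character's SpawnDartAtLocation and spawns a BP_DartNoPhysics, but the recorded positions are unused.
; Box1's overlap handler is empty, leaving disconnected dart-replacement logic.
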(event OnComponentBeginOverlap(Box1)
  (params (OverlappedComponent :type Primitive%20Component%20Object%20Reference) (OtherActor :type Actor%20Object%20Reference) (OtherComp :type Primitive%20Component%20Object%20Reference) (OtherBodyIndex :type Integer) (bFromSweep :type Boolean) (SweepResult :type Hit%20Result%20Structure%20%28by%20ref%29)))

(event Custom|NextBar
  (Variables|Default|SetRelative%20Location%20Z (Variables|/Game/Blueprints/BP_DartBar.BP_DartBar_C|GetRelative%20Location%20Z (Variables|Default|GetDartBar1)))
  (bind _asbp_dart_bar (Utilities|Casting|CastToBP_DartBar (Variables|/Script/Engine.ChildActorComponent|GetChildActor (Variables|Default|GetDartBarVert))))
  (bind _output_get (Variables|Default|SetDartBar2 _asbp_dart_bar))
  (Input|EnableInput _output_get (Game|GetPlayerController 0))
  (EventDispatchers|BindEventtoDone (Variables|Default|GetDartBar2) (delegate Custom|SpawnDart)))

(event Custom|SpawnDart
  (Variables|Default|SetRelative%20Location%20X (Variables|/Game/Blueprints/BP_DartBar.BP_DartBar_C|GetRelative%20Location%20Z (Variables|Default|GetDartBar2)))
  (bind _asbp_first_person_character (Utilities|Casting|CastToBP_FirstPersonCharacter (Game|GetPlayerCharacter 0)))
  (Default|SpawnDartatLocation _asbp_first_person_character 0.0 0.0)
  (Game|SpawnActorfromClass "/Game/Blueprints/BP_DartNoPhysics.BP_DartNoPhysics_C" (Math|Transform|MakeTransform "0, 0, 0" "0, 0, 0" "1.000000,1.000000,1.000000") "AlwaysSpawn" "MultiplyWithRoot" 0 0))

(event EventBeginPlay
  (bind _asbp_dart_bar (Utilities|Casting|CastToBP_DartBar (Variables|/Script/Engine.ChildActorComponent|GetChildActor (Variables|Default|GetDartBarHor))))
  (bind _output_get (Variables|Default|SetDartBar1 _asbp_dart_bar))
  (Input|EnableInput _output_get (Game|GetPlayerController 0))
  (EventDispatchers|BindEventtoDone (Variables|Default|GetDartBar1) (delegate Custom|NextBar)))

(fn ConstructionScript)